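; BPC_HealthComponent is an actor component that tracks its owner's health and death state.
; On BeginPlay it fills health to max and binds to the owner's OnTakeAnyDamage.
; Damage subtracts from health unclamped, prints the result, then broadcasts OnOwnerDamaged, or sets IsDead and broadcasts OnOwnerDied at zero or below.
; Getters expose health and death state; OwnerAlive is an unfinished stub that only casts the owner to BP_RootCharacter.
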(event Custom|DamageActor
  (params (DamagedActor :type Actor%20Object%20Reference) (Damage :type Float%20%28single-precision%29) (DamageType :type Damage%20Type%20Object%20Reference) (InstigatedBy :type Controller%20Object%20Reference) (DamageCauser :type Actor%20Object%20Reference))
  (bind _output_get (Variables|Private|SetCurrentHealth (- (Variables|Private|GetCurrentHealth) Damage)))
  (Development|PrintString (Utilities|String|ToString(Float) (Variables|Private|GetCurrentHealth)))
  (if (<= _output_get 0.0)
    (CallFunction|OwnerDied)
    (else
      (Default|CallOnOwnerDamaged))))

(event Custom|OwnerDied
  (Variables|Private|SetbIsDead true)
  (Default|CallOnOwnerDied))

(event Custom|OwnerAlive
  (bind _ownerref (Variables|Private|GetOwnerRef))
  (Utilities|IsValid _ownerref
    (:Is%20Valid
      (Utilities|Casting|CastToBP_RootCharacter _ownerref))))

(event EventBeginPlay
  (Variables|Private|SetCurrentHealth (Variables|Attributes|GetMaxHealth))
  (bind _output_get (Variables|Private|SetOwnerRef (Components|GetOwner)))
  (EventDispatchers|BindEventtoOnTakeAnyDamage _output_get (EventDispatchers|CreateEvent :!event Custom|DamageActor)))

(event EventTick
  (params (DeltaSeconds :type Float%20%28single-precision%29)))

(fn GetIsDead
  (return (Variables|Private|GetbIsDead)))

(fn GetHealth
  (return (Variables|Private|GetCurrentHealth)))