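; Weapon component that sets off an explosion centered on its owner, damaging surrounding actors that have a health component.
; Attack spends ammo and starts a timed cooldown, then plays particle, camera shake and sound effects at the owner's location.
; A zero-length multi-sphere object trace ignoring the owner finds the targets.
; IncrementAmmo, gated by a DoOnce, adds ammo and tells the owning BP_RootCharacter to update it.
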(event Custom|Attack
  (bind _ownerref (Variables|Private|GetOwnerRef))
  (bind _ownerref_2 (Variables|Private|GetOwnerRef))
  (bind _returnvalue (Transformation|GetActorLocation _ownerref))
  (bind _returnvalue_2 (Transformation|GetActorLocation _ownerref_2))
  (if (and (Variables|Private|GetbCanFire) (> (Variables|Private|GetAmmo) 0))
    (Utilities|Time|SetTimerbyEvent (EventDispatchers|CreateEvent :!event Custom|ResetCooldown) (Variables|Default|GetCooldown))
    (Variables|Private|SetbCanFire false)
    (Variables|Private|SetAmmo (- (Variables|Private|GetAmmo) 1))
    (Effects|SpawnEmitteratLocation "/Game/GrenadePack/Particles/VFX_GrenadeEXP_default.VFX_GrenadeEXP_default" _returnvalue_2)
    (Camera|PlayWorldCameraShake "/Game/Blueprints/Misc/BP_BombShake.BP_BombShake_C" _returnvalue_2 0.0 1e+04)
    (Audio|PlaySoundatLocation "/Game/Sound/Obstacles/explosion_Cue.explosion_Cue" _returnvalue_2 "0, 0, 0" 1.0 1.0 0.0 0 0 0)
    (bind _outhits (Collision|MultiSphereTraceForObjects _returnvalue _returnvalue (Variables|Default|GetRadius) (Utilities|Array|MakeArray "ObjectTypeQuery1" "ObjectTypeQuery2") false (Utilities|Array|MakeArray _ownerref) "None"))
    (for _array_element _outhits
      (Utilities|IsValid (Actor|GetComponentbyClass (.hitactor _array_element) "/Game/Blueprints/Components/BPC_HealthComponent.BPC_HealthComponent_C")
        (:Is%20Valid
          (Game|Damage|ApplyDamage (.hitactor _array_element) (Variables|Default|GetDamage) 0 0))))))

(event Custom|ResetCooldown
  (Variables|Private|SetbCanFire true))

(event EventBeginPlay
  (Variables|Private|SetOwnerRef (Components|GetOwner)))

(fn IncrementAmmo
  (Utilities|FlowControl|DoOnce false
    (:Completed
      (Variables|Private|SetAmmo (+ (Variables|Private|GetAmmo) 1))
      (bind _asbp_root_character (Utilities|Casting|CastToBP_RootCharacter (Variables|Private|GetOwnerRef)))
      (Default|UpdateAmmo _asbp_root_character))))

(fn GetAmmo
  (return (Variables|Private|GetAmmo)))