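; BP_RootGM, apparently the game mode, manages music playback and provides an event to open UI_TestingLevel.
; StartMusic plays a given 2D sound, then a duration-based timer calls HandleLoopingMusic to play the main or ending theme by MusicInt.
; At index zero that handler increments MusicInt and sets another timer.
; FadeOutMusic uses a timeline to drive the volume of the level's AmbientSound found at BeginPlay, printing each value.
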(event Custom|StartMusic
  (params (Sound :type Sound%20Base%20Object%20Reference))
  (Audio|PlaySound2D Sound 1.0 1.0 0.0 0 (Variables|Default|GetGameMusic))
  (Utilities|Time|SetTimerbyEvent (delegate Custom|HandleLoopingMusic) (Variables|/Script/Engine.SoundBase|GetDuration Sound)))

(event Custom|HandleLoopingMusic
  (bind _musicint (Variables|Default|GetMusicInt))
  (bind _returnvalue (Utilities|Select :Index _musicint :Option%200 "/Game/Music/GGJ_RootIndustrial_-_main_theme.GGJ_RootIndustrial_-_main_theme" :Option%201 "/Game/Music/GGJ_RootIndustrial_-_ending.GGJ_RootIndustrial_-_ending"))
  (Audio|PlaySound2D _returnvalue 1.0 1.0 0.0 0 (Variables|Default|GetGameMusic))
  (if (== (Variables|Default|GetMusicInt) 0)
    (Math|Integer|IncrementInt (Variables|Default|GetMusicInt)
      (:%20%20
        (Utilities|Time|SetTimerbyEvent (EventDispatchers|CreateEvent :!event Custom|HandleLoopingMusic) (Variables|/Script/Engine.SoundBase|GetDuration _returnvalue))))))

(event Custom|FadeOutMusic
  (bind _newtrack_0 (Timeline|Timeline_0 PlayFromStart)
    (:Update
      (Audio|Components|Audio|SetVolumeMultiplier (Variables|/Script/Engine.AmbientSound|GetAudioComponent (Variables|Default|GetGameMusic)) _newtrack_0 :!class /Script/Engine.AudioComponent)
      (Development|PrintString (Utilities|String|ToString(Float) _newtrack_0)))))

(event Custom|LoadLevel
  (Game|OpenLevel(byName) "UI_TestingLevel"))

(event EventBeginPlay
  (bind _returnvalue (Actor|GetActorOfClass "/Script/Engine.AmbientSound"))
  (bind _output_get (Variables|Default|SetGameMusic _returnvalue))
  (Audio|Components|Audio|SetVolumeMultiplier (Variables|/Script/Engine.AmbientSound|GetAudioComponent _output_get) 1.0 :!class /Script/Engine.AudioComponent))

(event EventTick
  (params (DeltaSeconds :type Float%20%28single-precision%29)))

(fn ConstructionScript)