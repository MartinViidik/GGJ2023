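; Player character for a descending game: it falls at PlayerSpeed per tick while steering sideways and attacking through a weapon component.
; Any key press creates the HUD and, if alive and not moving, starts descent, light fade-in and camera intro.
; Health component events update the HUD on damage; death stops movement and fades out the light.
; Distance traveled supplies the score in meters, and an exposed modifier adjusts speed.
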(event OnOwnerDamaged(BPC_HealthComponent)
  (Default|SetCurrentHealth (Variables|Default|GetHUD) (Default|GetHealth (Variables|Default|GetBPC_HealthComponent))))

(event OnOwnerDied(BPC_HealthComponent)
  ;[1 1 1] Player Health
  (CallFunction|SetPlayerMovement false)
  (Pawn|Components|CharacterMovement|DisableMovement (Variables|Character|GetCharacterMovement))
  (CallFunction|PlayLight true))

(event Custom|SetPlayerMovement
  (params (bEnabled :type Boolean))
  ;[1 1 1] Character Movement
  (Actor|Tick|SetActorTickEnabled bEnabled))

(event EventTick
  (params (DeltaSeconds :type Float%20%28single-precision%29))
  ;[1 1 1] Character Movement
  (CallFunction|MovePlayerDown))

(event Input|AxisEvents|InputAxisMoveRight
  (params (AxisValue :type Float%20%28single-precision%29))
  ;[1 1 1] Character Movement
  (Pawn|Input|AddMovementInput (Math|Vector|GetRightVector (Variables|Default|GetCamera)) AxisValue false))

(event Input|KeyboardEvents|AnyKey
  (params (Key :type Key%20Structure :default "None"))
  (:Pressed
    (CallFunction|HandleGameStart)
    (bind _returnvalue (UserInterface|CreateWidget "/Game/Blueprints/UI/BP_GameHUD.BP_GameHUD_C"))
    (UserInterface|Viewport|AddtoViewport _returnvalue 0)
    (Variables|Default|SetHUD _returnvalue)))

(event Input|KeyboardEvents|SpaceBar
  (params (Key :type Key%20Structure :default "None"))
  (:Pressed
    (Default|Attack (Variables|Default|GetBPC_Weapon))))

(event Custom|PlayLight
  (params (bReverse :type Boolean))
  ;[1 1 1] Cosmetic functions
  (if bReverse
    (bind _newtrack_0 (Timeline|ControlLight ReverseFromEnd)
      (:Update
        (Rendering|Components|Light|SetIntensity (Variables|Default|GetPointLight) (Math|Float|Lerp 0.0 (Variables|Default|GetLightIntensity) _newtrack_0))))
    (else
      (Timeline|ControlLight PlayFromStart))))

(event Custom|StartingCamera
  ;[1 1 1] Cosmetic functions
  (Components|Timeline|SetPlayRate (Variables|Default|GetMoveCamera) 0.15)
  (bind _newtrack_0 (Timeline|MoveCamera Play)
    (:Update
      (Transformation|SetRelativeRotation (Variables|Default|GetCamera) (Math|Rotator|Lerp(Rotator) "20.000000, 0, 0" "0, 0, 0" _newtrack_0) false false)
      (Transformation|SetRelativeRotation (Variables|Default|GetSpringArm) (Math|Rotator|Lerp(Rotator) "-20.000000, 0, 0" "0, 0, 0" _newtrack_0) false false))))

(fn ConstructionScript)

(fn MovePlayerDown
  (Transformation|SetActorLocation (- (Transformation|GetActorLocation) (Math|Vector|MakeVector 0.0 0.0 (Variables|Default|GetPlayerSpeed))) false false)
  (Variables|Default|SetDistanceTraveled (+ (Variables|Default|GetDistanceTraveled) (Variables|Default|GetPlayerSpeed))))

(fn HandleGameStart
  (if (and (not (Default|GetIsDead (Variables|Default|GetBPC_HealthComponent))) (not (Class|Actor|IsActorTickEnabled)))
    (CallFunction|SetPlayerMovement true)
    (CallFunction|PlayLight false)
    (Components|Timeline|SetPlayRate (Variables|Default|GetControlLight) 3.0)
    (CallFunction|StartingCamera)))

(fn ModifyCharacterSpeed
  (params (Modifier :type Float%20%28single-precision%29))
  (Variables|Default|SetPlayerSpeed (+ (Variables|Default|GetPlayerSpeed) Modifier)))

(fn GetScore
  (return (Utilities|Text|FormatText "{amount}m" (Math|Float|Round (/ (Variables|Default|GetDistanceTraveled) 1e+01)))))