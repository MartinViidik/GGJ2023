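; Base pickup actor for powerups that reacts when something overlaps its sphere.
; An overlapping BP_RootCharacter triggers ApplyEffect, which in this base only calls StartScale, while any other actor destroys the pickup immediately.
; StartScale plays the ScaleDown timeline, shrinking the mesh from its scale cached at BeginPlay to zero, then destroys the pickup.
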(event OnComponentBeginOverlap(Sphere)
  (params (OverlappedComponent :type Primitive%20Component%20Object%20Reference) (OtherActor :type Actor%20Object%20Reference) (OtherComp :type Primitive%20Component%20Object%20Reference) (OtherBodyIndex :type Integer) (bFromSweep :type Boolean) (SweepResult :type Hit%20Result%20Structure%20%28by%20ref%29))
  (Utilities|Casting|CastToBP_RootCharacter OtherActor
    (:then
      (CallFunction|ApplyEffect OtherActor))
    (:CastFailed
      (Actor|DestroyActor))))

(event Custom|ApplyEffect
  (params (TargetActor :type Actor%20Object%20Reference))
  (CallFunction|StartScale))

(event Custom|StartScale
  (bind _alpha (Timeline|ScaleDown Play)
    (:Update
      (Transformation|SetWorldScale3D (Variables|Default|GetStaticMesh) (Math|Vector|Lerp(Vector) (Variables|Default|GetCacheScale) "0, 0, 0" _alpha)))
    (:Finished
      (Actor|DestroyActor))))

(event EventBeginPlay
  (Variables|Default|SetCacheScale (Transformation|GetWorldScale (Variables|Default|GetStaticMesh))))

(fn ConstructionScript)