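; BP_BombImpact is a one-shot destructible obstacle actor that shatters as soon as it spawns.
; On BeginPlay it applies random damage and impulse to its Destructible component, using the actor location as both hit point and impulse direction.
; It then enables gravity on the component, disables actor collision, plays a rock rubble sound and destroys itself after a short delay.
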(event EventBeginPlay
  (bind _returnvalue (Transformation|GetActorLocation))
  (bind _returnvalue_2 (Math|Random|RandomFloatinRange 1e+03 5e+03))
  (Class|DestructibleComponent|ApplyDamage (Variables|Default|GetDestructible) _returnvalue_2 _returnvalue _returnvalue _returnvalue_2)
  (Physics|SetEnableGravity (Variables|Default|GetDestructible) true)
  (Collision|SetActorEnableCollision false)
  (Audio|PlaySoundatLocation "/Game/Sound/Obstacles/S_RockRubble03_Cue.S_RockRubble03_Cue" (Transformation|GetActorLocation) "0, 0, 0" 1.0 1.0 0.0 0 0 0)
  (Utilities|FlowControl|Delay 3.0)
  (Actor|DestroyActor))

(fn ConstructionScript)