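; BP_Rock is an obstacle actor that gives each placed rock a randomized look.
; Its construction script calls the parent script, then applies a random per-axis scale within a narrow range and a random rotation without roll to the static mesh.
; It also picks a random mesh from the RockModels array, so the variation is set at construction while the event graph holds no active logic.
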(event EventBeginPlay)

(event Collision|EventActorBeginOverlap
  (params (OtherActor :type Actor%20Object%20Reference)))

(event EventTick
  (params (DeltaSeconds :type Float%20%28single-precision%29)))

(fn ConstructionScript
  (bind _returnvalue (Math|Random|RandomFloatinRange 0.45 0.6))
  (bind _rockmodels (Variables|Default|GetRockModels))
  (|CallParentFunction)
  (Transformation|SetWorldScale3D (Variables|Default|GetStaticMesh) (Math|Vector|MakeVector _returnvalue _returnvalue _returnvalue))
  (Transformation|SetWorldRotation (Variables|Default|GetStaticMesh) (Math|Random|RandomRotator false) false false)
  (Components|StaticMesh|SetStaticMesh (Variables|Default|GetStaticMesh) (Utilities|Array|Get(acopy) _rockmodels (.OutIndex (Utilities|Array|Random _rockmodels)))))