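; BP_TutorialText is a world actor that shows tutorial text while a BP_RootCharacter is inside its collision volume.
; On BeginPlay it creates a dynamic material instance on TutorialText and sets its Opacity to zero.
; Begin and end overlap call SetTextState, which plays or reverses the FadeText timeline to drive Opacity, fading the text in on entry and out on exit.
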(event OnComponentBeginOverlap(Collision)
  (params (OverlappedComponent :type Primitive%20Component%20Object%20Reference) (OtherActor :type Actor%20Object%20Reference) (OtherComp :type Primitive%20Component%20Object%20Reference) (OtherBodyIndex :type Integer) (bFromSweep :type Boolean) (SweepResult :type Hit%20Result%20Structure%20%28by%20ref%29))
  (Utilities|Casting|CastToBP_RootCharacter OtherActor)
  (CallFunction|SetTextState false))

(event OnComponentEndOverlap(Collision)
  (params (OverlappedComponent :type Primitive%20Component%20Object%20Reference) (OtherActor :type Actor%20Object%20Reference) (OtherComp :type Primitive%20Component%20Object%20Reference) (OtherBodyIndex :type Integer))
  (Utilities|Casting|CastToBP_RootCharacter OtherActor)
  (CallFunction|SetTextState true))

(event Custom|SetTextState
  (params (bFade :type Boolean))
  (if bFade
    (bind _alpha (Timeline|FadeText Reverse)
      (:Update
        (Rendering|Material|SetScalarParameterValue (Variables|Default|GetTextMaterial) "Opacity" _alpha :!class /Script/Engine.MaterialInstanceDynamic)))
    (else
      (Timeline|FadeText Play))))

(event EventBeginPlay
  (bind _returnvalue (Rendering|Material|CreateDynamicMaterialInstance (Variables|Default|GetTutorialText) 0 (Rendering|Material|GetMaterial (Variables|Default|GetTutorialText) 0) "None" :!class /Script/Engine.PrimitiveComponent))
  (bind _output_get (Variables|Default|SetTextMaterial _returnvalue))
  (Rendering|Material|SetScalarParameterValue _output_get "Opacity" 0.0 :!class /Script/Engine.MaterialInstanceDynamic))

(event Collision|EventActorBeginOverlap
  (params (OtherActor :type Actor%20Object%20Reference)))

(event EventTick
  (params (DeltaSeconds :type Float%20%28single-precision%29)))

(fn ConstructionScript)